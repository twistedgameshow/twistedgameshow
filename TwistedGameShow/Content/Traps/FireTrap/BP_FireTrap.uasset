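; Fire trap that follows a linked Activator's IsActivated state and reports a kill when the player is in its box while it burns.
; Tick polls the Activator, using paired DoOnce gates to switch four fire particle systems on or off only on state changes.
; Construction starts the fire disabled.
; Box overlap tracks the first-person player; the kill is only a one-time "Player killed" print, with no damage applied.
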(event `self.ReceiveTick`
  (params (DeltaSeconds :type "Float (single-precision)"))
  (bind _activator (`self.Activator`))
  (`|ExecutionSequence`
    (:`then_0`
      (`/Engine/EditorBlueprintResources/StandardMacros.IsValid` _activator
        (:`Is Valid`
          (if (`/Game/PlayerInteractables/BP_BasePlayerInteractable.isActivated` _activator)
            (`|ExecutionSequence`
              (:`then_0`
                (`/Engine/EditorBlueprintResources/StandardMacros.DoOnce` false :!label _label
                  (:`Completed`
                    (`self.EnableFire`)
                    (set `self.FireOn` true))))
              (:`then_1`
                (goto _label_2 :!via `Reset`)))
            (else
              (`|ExecutionSequence`
                (:`then_0`
                  (goto _label :!via `Reset`))
                (:`then_1`
                  (`/Engine/EditorBlueprintResources/StandardMacros.DoOnce` false :!label _label_2
                    (:`Completed`
                      (`self.DisableFire`)
                      (set `self.FireOn` false))))))))))
    (:`then_1`
      (if (and (`self.PlayerInRadius`) (`self.FireOn`))
        (`/Engine/EditorBlueprintResources/StandardMacros.DoOnce` false
          (:`Completed`
            (cast `/Game/FirstPersonBP/Blueprints/FirstPersonCharacter` (`GameplayStatics.GetPlayerPawn` 0))
            (`KismetSystemLibrary.PrintString` "Player killed")))))))

(event `self.Box.OnComponentBeginOverlap`
  (params (OverlappedComponent :type "PrimitiveComponent Object Reference") (OtherActor :type "Actor Object Reference") (OtherComp :type "PrimitiveComponent Object Reference") (OtherBodyIndex :type Integer) (bFromSweep :type Boolean) (SweepResult :type "HitResult Structure (by ref)"))
  (cast `/Game/FirstPersonBP/Blueprints/FirstPersonCharacter` OtherActor)
  (set `self.PlayerInRadius` true))

(event `self.ReceiveActorEndOverlap`
  (params (OtherActor :type "Actor Object Reference"))
  (cast `/Game/FirstPersonBP/Blueprints/FirstPersonCharacter` OtherActor)
  (set `self.PlayerInRadius` false))

(fn `DisableFire`
  (for _array_element (`|MakeArray` "Flames" "Smoke" "Embers" "Sparks" "Distortion" :!type "Name")
    (`ParticleSystemComponent.SetEmitterEnable` (`self.Fire2`) _array_element false)
    (`ParticleSystemComponent.SetEmitterEnable` (`self.Fire3`) _array_element false)
    (`ParticleSystemComponent.SetEmitterEnable` (`self.Fire4`) _array_element false)
    (`ParticleSystemComponent.SetEmitterEnable` (`self.Fire1`) _array_element false)))

(fn `EnableFire`
  (for _array_element (`|MakeArray` "Flames" "Smoke" "Embers" "Sparks" "Distortion" :!type "Name")
    (`ParticleSystemComponent.SetEmitterEnable` (`self.Fire2`) _array_element true)
    (`ParticleSystemComponent.SetEmitterEnable` (`self.Fire3`) _array_element true)
    (`ParticleSystemComponent.SetEmitterEnable` (`self.Fire4`) _array_element true)
    (`ParticleSystemComponent.SetEmitterEnable` (`self.Fire1`) _array_element true)))

(fn `UserConstructionScript`
  (`self.DisableFire`))