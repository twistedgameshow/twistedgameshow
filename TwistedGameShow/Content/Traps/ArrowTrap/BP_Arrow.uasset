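; Arrow trap projectile that spins around its roll axis in flight and kills the first-person player on impact.
; On its first hit it spawns a movable, collision-free static mesh copy of the arrow attached to whatever it struck, then destroys itself.
; The stuck copy is tagged KillOnCheckpoint, and a player hit triggers KillPlayer on the character.
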(event `self.ReceiveTick`
  (params (DeltaSeconds :type "Float (single-precision)"))
  (if (not (`ProjectileMovementComponent.IsVelocityUnderSimulationThreshold` (`self.ProjectileMovement`)))
    (`self.K2_AddActorLocalRotation` (`KismetMathLibrary.MakeRotator` (* DeltaSeconds 5000.0)))))

(event `self.ReceiveHit`
  (params (MyComp :type "PrimitiveComponent Object Reference") (Other :type "Actor Object Reference") (OtherComp :type "PrimitiveComponent Object Reference") (bSelfMoved :type Boolean) (HitLocation :type "Vector Structure") (HitNormal :type "Vector Structure") (NormalImpulse :type "Vector Structure") (Hit :type "HitResult Structure (by ref)"))
  (if (not (`self.hit?`))
    (set `self.hit?` true)
    (`KismetSystemLibrary.PrintString` "Arrow Hit")
    (bind _returnvalue (`|SpawnActorFromClass` "/Script/Engine.StaticMeshActor" (`self.GetTransform` self) "AdjustIfPossibleButAlwaysSpawn" "OverrideRootScale" null null))
    (`StaticMeshActor.SetMobility` _returnvalue "Movable")
    (set `Actor.Tags` (`|MakeArray` "KillOnCheckpoint" :!type "Name") _returnvalue)
    (bind _staticmeshcomponent (`StaticMeshActor.StaticMeshComponent` _returnvalue))
    (`StaticMeshComponent.SetStaticMesh` _staticmeshcomponent "/Game/Traps/ArrowTrap/Meshes/Arrow.Arrow")
    (`PrimitiveComponent.SetCollisionEnabled` _staticmeshcomponent "NoCollision")
    (`self.K2_AttachToActor` _returnvalue Other "None" "KeepWorld" "KeepWorld" "KeepWorld" true)
    (bind _asfirst_person_character (cast `/Game/FirstPersonBP/Blueprints/FirstPersonCharacter` Other)
      (:`then`
        (`/Game/FirstPersonBP/Blueprints/FirstPersonCharacter.Kill Player ` _asfirst_person_character))
      (:`CastFailed`
        _))
    (`self.K2_DestroyActor`)))

(fn `UserConstructionScript`)