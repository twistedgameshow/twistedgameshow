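; Arrow trap that spawns BP_Arrow projectiles from two spawn points.
; FireArrows runs on BeginPlay and again when Tick first sees TriggerInteractable activated, gated by a DoOnce.
; It splits the ArrowsToSpawn count between Spawn1 and Spawn2, spawning at their world transforms, then hides the Arrow1 and Arrow2 components.
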(event `self.ReceiveBeginPlay`
  (`self.FireArrows` :!label _label))

(event `self.ReceiveTick`
  (params (DeltaSeconds :type "Float (single-precision)"))
  (if (`/Game/PlayerInteractables/BP_BasePlayerInteractable.isActivated` (`self.TriggerInteractable`))
    (`/Engine/EditorBlueprintResources/StandardMacros.DoOnce` false
      (:`Completed`
        (goto _label)))))

(event `FireArrows`
  (for _array_element (`|MakeArray` (`self.Spawn1`) (`self.Spawn2`))
    (for _ (range (+ (/ (`self.ArrowsToSpawn`) 2) 1))
      (`|SpawnActorFromClass` "/Game/Traps/ArrowTrap/BP_Arrow.BP_Arrow_C" (`SceneComponent.K2_GetComponentToWorld` _array_element) "AdjustIfPossibleButAlwaysSpawn" "OverrideRootScale" null null)))
  (`SceneComponent.SetVisibility` (`self.Arrow1`) false false)
  (`SceneComponent.SetVisibility` (`self.Arrow2`) false false))

(fn `UserConstructionScript`)