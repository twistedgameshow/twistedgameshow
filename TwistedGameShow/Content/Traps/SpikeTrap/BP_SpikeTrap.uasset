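; BP_SpikeTrap is a trap that raises spikes and kills the first-person player on contact.
; Tick polls a linked TriggerInteractable and fires the spikes once per activation through a DoOnce that resets on deactivation.
; Spikes rise quickly with collision disabled, re-enable collision, pause briefly, then retract more slowly.
; Actor overlaps call KillPlayer only while the Spiking flag is set, which clears before retraction.
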(event `self.ReceiveTick`
  (params (DeltaSeconds :type "Float (single-precision)"))
  (bind _trigger_interactable (`self.Trigger Interactable`))
  (`/Engine/EditorBlueprintResources/StandardMacros.IsValid` _trigger_interactable
    (:`Is Valid`
      (if (`/Game/PlayerInteractables/BP_BasePlayerInteractable.isActivated` _trigger_interactable)
        (`/Engine/EditorBlueprintResources/StandardMacros.DoOnce` false :!label _label
          (:`Completed`
            (`self.ActivateSpikes`)))
        (else
          (goto _label :!via `Reset`))))))

(event `ActivateSpikes`
  (bind _spikemesh (`self.SpikeMesh`))
  (set `self.Spiking` true)
  (`PrimitiveComponent.SetCollisionEnabled` _spikemesh "NoCollision")
  (`KismetSystemLibrary.MoveComponentTo` _spikemesh (0.0 0.0 0.0) (struct) false true 0.1)
  (`PrimitiveComponent.SetCollisionEnabled` _spikemesh "QueryAndPhysics")
  (`KismetSystemLibrary.Delay` 0.5)
  (set `self.Spiking` false)
  (`KismetSystemLibrary.MoveComponentTo` _spikemesh (0.0 0.0 -273.140015) (struct) true true 0.5))

(event `self.ReceiveActorBeginOverlap`
  (params (OtherActor :type "Actor Object Reference"))
  (if (`self.Spiking`)
    (bind _asfirst_person_character (cast `/Game/FirstPersonBP/Blueprints/FirstPersonCharacter` OtherActor))
    (`/Game/FirstPersonBP/Blueprints/FirstPersonCharacter.Kill Player ` _asfirst_person_character)))

(fn `UserConstructionScript`)