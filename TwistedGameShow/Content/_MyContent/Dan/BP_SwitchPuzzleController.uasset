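; Controller for a three-switch puzzle that opens a door when the switches are activated in the correct order.
; CheckSwitchStates advances a step enum as each switch combination matches, then opens the door and adds an audio component.
; Wrong presses in the first two steps fire spike traps if CanKill is set; otherwise, and always in step three, switches reset.
; Once done, all switches are forced on.
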(event `self.ReceiveTick`
  (params (DeltaSeconds :type "Float (single-precision)")))

(fn `CheckSwitchStates`
  (bind _switch_1 (`self.Switch 1`))
  (bind _switch_2 (`self.Switch 2`))
  (bind _switch_2_2 (`self.Switch 2`))
  (bind _switch_3 (`self.Switch 3`))
  (bind _switch_1_2 (`self.Switch 1`))
  (bind _switch_3_2 (`self.Switch 3`))
  (bind _isactivated (`/Game/PlayerInteractables/BP_BasePlayerInteractable.isActivated` _switch_1))
  (bind _isactivated_2 (`/Game/PlayerInteractables/BP_BasePlayerInteractable.isActivated` _switch_2_2))
  (switch `/Game/_MyContent/Dan/ENUM_SwitchPuzzle` (`self.PuzzleStep`)
    (:`NewEnumerator0`
      ;[1 1 1] Check if first switch has been pressed
      (if _isactivated
        (set `self.PuzzleStep` "NewEnumerator1")
        (elif (`self.Can Kill`)
          (for _array_element (`self.Traps`)
            (`/Game/Traps/SpikeTrap/BP_SpikeTrap.ActivateSpikes` _array_element))
          (else
            (`/Game/PlayerInteractables/BP_BasePlayerInteractable.Deactivate` _switch_2_2)
            (`/Game/PlayerInteractables/BP_BasePlayerInteractable.Deactivate` _switch_3)))))
    (:`NewEnumerator1`
      ;[1 1 1] Check if second switch combination is correct
      (if (and _isactivated _isactivated_2)
        (set `self.PuzzleStep` "NewEnumerator2")
        (elif (`self.Can Kill`)
          (for _array_element_2 (`self.Traps`)
            (`/Game/Traps/SpikeTrap/BP_SpikeTrap.ActivateSpikes` _array_element_2))
          (else
            (`/Game/PlayerInteractables/BP_BasePlayerInteractable.Deactivate` _switch_1 :!label _label)
            (`/Game/PlayerInteractables/BP_BasePlayerInteractable.Deactivate` _switch_2_2)
            (`/Game/PlayerInteractables/BP_BasePlayerInteractable.Deactivate` _switch_3)
            (set `self.PuzzleStep` "NewEnumerator0")))))
    (:`NewEnumerator2`
      ;[1 1 1] Check 3rd correct switch is pressed
      (if (and _isactivated _isactivated_2 (`/Game/PlayerInteractables/BP_BasePlayerInteractable.isActivated` _switch_3))
        (`/Game/DoorsAndKeys/BP_DoorWithFunction.DoorOpenFunction` (`self.Door`))
        (set `self.PuzzleStep` "NewEnumerator3")
        (`AddComponent|NODE_AddAudioComponent-0`)
        (else
          (goto _label))))
    (:`NewEnumerator3`
      (set `/Game/PlayerInteractables/BP_BasePlayerInteractable.isActivated` true _switch_1_2)
      (`/Game/PlayerInteractables/BP_BasePlayerInteractable.UpdateAfterChange` _switch_1_2)
      (set `/Game/PlayerInteractables/BP_BasePlayerInteractable.isActivated` true _switch_2)
      (`/Game/PlayerInteractables/BP_BasePlayerInteractable.UpdateAfterChange` _switch_2)
      (set `/Game/PlayerInteractables/BP_BasePlayerInteractable.isActivated` true _switch_3_2)
      (`/Game/PlayerInteractables/BP_BasePlayerInteractable.UpdateAfterChange` _switch_3_2))))

(fn `UserConstructionScript`)