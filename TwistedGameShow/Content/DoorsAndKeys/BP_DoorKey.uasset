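; BP_DoorKey is a locked door that the player opens with G once they hold the matching key.
; On box overlap, it scans the FirstPersonCharacter's Key array and enables input on the door if the entry at index DoorValue is true.
; Pressing G plays a timeline that moves DoorMesh's relative location.
; The graph never disables input or reverses the movement.
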(event `self.Box.OnComponentBeginOverlap`
  (params (OverlappedComponent :type "PrimitiveComponent Object Reference") (OtherActor :type "Actor Object Reference") (OtherComp :type "PrimitiveComponent Object Reference") (OtherBodyIndex :type Integer) (bFromSweep :type Boolean) (SweepResult :type "HitResult Structure (by ref)"))
  (bind _asfirst_person_character (cast `/Game/FirstPersonBP/Blueprints/FirstPersonCharacter` OtherActor))
  (for (_array_element _array_index) (`/Game/FirstPersonBP/Blueprints/FirstPersonCharacter.Key` _asfirst_person_character)
    (if (and _array_element (== _array_index (`self.Door Value`)))
      (`self.EnableInput` (`GameplayStatics.GetPlayerController` 0)))))

(event `Key|G`
  (params (Key :type "Key Structure"))
  (:`Pressed`
    (bind (_direction _newtrack_0) (`Timeline|Timeline_0`)
      (:`Update`
        (`SceneComponent.K2_SetRelativeLocation` (`self.Door Mesh`) _newtrack_0 false false)))))

(fn `UserConstructionScript`)