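; Checkpoint save and load functions that snapshot the world to a save slot and restore it.
; Save records player transform, static mesh transforms and physics, and interactable states; timer and arrow trap data are gathered but never written to the save object.
; Load matches actors by object name, restores their state and any valid timer data.
; It then resets arrow traps and destroys actors tagged KillOnCheckpoint.
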(fn `LoadAbsolutleyEverything`
  (locals (LoadableInteractables :type "Array of /Game/PlayerInteractables/BP_BasePlayerInteractable Object Reference") (LoadableStaticMeshes :type "Array of StaticMeshActor Object Reference") (LoadableArrowTraps :type "Array of /Game/Traps/ArrowTrap/BP_ArrowTrap Object Reference"))
  (`KismetSystemLibrary.PrintString` null "Loading...")
  (bind _returnvalue (`GameplayStatics.LoadGameFromSlot` "saved_world" 1))
  (`/Engine/EditorBlueprintResources/StandardMacros.IsValid` _returnvalue
    (:`Is Valid`
      (bind _outactors (`GameplayStatics.GetAllActorsOfClass` null "/Game/Traps/ArrowTrap/BP_ArrowTrap.BP_ArrowTrap_C"))
      (set `local.LoadableArrowTraps` _outactors)
      (bind _outactors_2 (`GameplayStatics.GetAllActorsOfClass` null "/Script/Engine.StaticMeshActor"))
      (set `local.LoadableStaticMeshes` _outactors_2)
      (bind _outactors_3 (`GameplayStatics.GetAllActorsOfClass` null "/Game/PlayerInteractables/BP_BasePlayerInteractable.BP_BasePlayerInteractable_C"))
      (set `local.LoadableInteractables` _outactors_3)
      (bind _asbp_tgs_checkpoint_save_game (cast `/Game/Checkpoints/BP_TGS_Checkpoint_SaveGame` _returnvalue)
        (:`then`
          (`|ExecutionSequence`
            (:`then_0`
              (bind _player_data (`/Game/Checkpoints/BP_TGS_Checkpoint_SaveGame.Player Data` _asbp_tgs_checkpoint_save_game))
              ;[1 1 1] Load player position and set
              (if (`.ValidData_8_8E7E41344BE86A2EF187A1B021BCD2D2` (break `/Game/Checkpoints/EmbeddedData/S_PlayerData` _player_data))
                (`Actor.K2_SetActorLocationAndRotation` (`GameplayStatics.GetPlayerPawn` null) (.location (break `/Game/Checkpoints/EmbeddedData/S_PlayerData` _player_data)) (.rotation (break `/Game/Checkpoints/EmbeddedData/S_PlayerData` _player_data)) false false)
                (if (!= (.scale (break `/Game/Checkpoints/EmbeddedData/S_PlayerData` _player_data)) (1.0 1.0 1.0))
                  (`KismetSystemLibrary.PrintString` null "Player scale is not 1. What are you doing?"))
                (else
                  (`KismetSystemLibrary.PrintString` null "Invalid player data, skipping load."))))
            (:`then_1`
              ;[1 1 1] Load Mesh States
              (for _array_element (`/Game/Checkpoints/BP_TGS_Checkpoint_SaveGame.NonStatic Meshes` _asbp_tgs_checkpoint_save_game)
                (for _array_element_2 (`local.LoadableStaticMeshes`)
                  (bind _returnvalue_2 (`KismetSystemLibrary.GetObjectName` _array_element_2))
                  (if (and (`KismetStringLibrary.EqualEqual_StrStr` _returnvalue_2 (break `/Game/Checkpoints/EmbeddedData/S_PhysicsMesh_Data` _array_element)) (`.ValidData_15_5B124D4A435B960091E346B5266F1204` (break `/Game/Checkpoints/EmbeddedData/S_PhysicsMesh_Data` _array_element)))
                    (`|ExecutionSequence`
                      (:`then_0`
                        (`Actor.K2_SetActorTransform` _array_element_2 (`.Transform_2_736C5D1E4328296247AD76939A627FF1` (break `/Game/Checkpoints/EmbeddedData/S_PhysicsMesh_Data` _array_element)) false true))
                      (:`then_1`
                        (bind _staticmeshcomponent (`StaticMeshActor.StaticMeshComponent` _array_element_2))
                        (`PrimitiveComponent.SetSimulatePhysics` _staticmeshcomponent (`.SimPhysics_8_66B92D844849E4B8DB613DA57418319C` (break `/Game/Checkpoints/EmbeddedData/S_PhysicsMesh_Data` _array_element))))
                      (:`then_2`
                        (`PrimitiveComponent.SetPhysicsLinearVelocity` _staticmeshcomponent (`.Velocity_11_B50F3ECD48F3455719DCA19AF8DFF1ED` (break `/Game/Checkpoints/EmbeddedData/S_PhysicsMesh_Data` _array_element)) false "None"))
                      (:`then_3`
                        (`KismetSystemLibrary.PrintString` null (`KismetStringLibrary.Concat_StrStr` "Loading " _returnvalue_2)))
                      (:`then_4`
                        (break)))))))
            (:`then_2`
              ;[1 1 1] Load Interactable states
              (for _array_element_3 (`/Game/Checkpoints/BP_TGS_Checkpoint_SaveGame.Interactables` _asbp_tgs_checkpoint_save_game)
                (for _array_element_4 (`local.LoadableInteractables`)
                  (if (and (`KismetStringLibrary.EqualEqual_StrStr` (`KismetSystemLibrary.GetObjectName` _array_element_4) (break `/Game/Checkpoints/EmbeddedData/S_Interactable_Data` _array_element_3)) (`.ValidData_8_942E1D23459F67B7D5CE2181FC161FE1` (break `/Game/Checkpoints/EmbeddedData/S_Interactable_Data` _array_element_3)))
                    (`/Game/PlayerInteractables/BP_BasePlayerInteractable.SetActivated` _array_element_4 (`.State_1_F934015E402D2A7D8F31538A95D6BDC6` (break `/Game/Checkpoints/EmbeddedData/S_Interactable_Data` _array_element_3)))
                    (break)))))
            (:`then_3`
              (bind _asbp_my_game_mode (cast `/Game/UI/BP_MyGameMode` (`GameplayStatics.GetGameMode` null)))
              (bind (_timerdata_minutes _timerdata_seconds _timerdata_secondsfrac _timerdata_valid) (break `/Game/Checkpoints/EmbeddedData/S_TimerSaveData` (`/Game/Checkpoints/BP_TGS_Checkpoint_SaveGame.TimerData` _asbp_tgs_checkpoint_save_game)))
              (if _timerdata_valid
                (set `/Game/UI/BP_MyGameMode.Minutes` _timerdata_minutes _asbp_my_game_mode)
                (set `/Game/UI/BP_MyGameMode.Seconds` _timerdata_seconds _asbp_my_game_mode)))
            (:`then_4`
              (`KismetSystemLibrary.PrintString` null "Done!"))
            (:`then_5`
              ;[1 1 1] Clean up arrow traps.
              (`|ExecutionSequence`
                (:`then_0`
                  (bind _outactors_4 (`GameplayStatics.GetAllActorsOfClass` null "/Game/Traps/ArrowTrap/BP_ArrowTrap.BP_ArrowTrap_C"))
                  (for _array_element_5 _outactors_4
                    (`/Game/Traps/ArrowTrap/BP_ArrowTrap.CheckpointReset` _array_element_5)))
                (:`then_1`
                  (bind _outactors_5 (`GameplayStatics.GetAllActorsWithTag` null "KillOnCheckpoint"))
                  (for _array_element_6 _outactors_5
                    (`Actor.K2_DestroyActor` _array_element_6)))))))
        (:`CastFailed`
          (`KismetSystemLibrary.PrintString` null "A ReAlLy BaD ErRoR occured when loading save game!!!!!!!!!!!!!!!!!!!!!!!" true true (struct :`R` 1.0 :`A` 1.0)))))
    (:`Is Not Valid`
      (`KismetSystemLibrary.PrintString` null "Error Loading!" true true (struct :`R` 1.0 :`G` 0.038292 :`A` 1.0)))))

(fn `SaveAbsolutleyEverything`
  (locals (`Player Data` :type "/Game/Checkpoints/EmbeddedData/S_PlayerData Structure") (Interactables :type "Array of /Game/Checkpoints/EmbeddedData/S_Interactable_Data Structure") (MovableMeshes :type "Array of /Game/Checkpoints/EmbeddedData/S_PhysicsMesh_Data Structure") (timeSave :type "/Game/Checkpoints/EmbeddedData/S_TimerSaveData Structure") (ArrowTrapSaves :type "Array of /Game/Checkpoints/EmbeddedData/S_ArrowTrapData Structure"))
  (`KismetSystemLibrary.PrintString` null "Checkpoint...")
  (`|ExecutionSequence`
    (:`then_0`
      ;[1 1 1] Serialize player data
      (bind _asfirst_person_character (cast `/Game/FirstPersonBP/Blueprints/FirstPersonCharacter` (`GameplayStatics.GetPlayerPawn` null))
        (:`then`
          (set `local.Player Data` (make `/Game/Checkpoints/EmbeddedData/S_PlayerData` (`Actor.GetTransform` _asfirst_person_character) (`KismetSystemLibrary.GetDisplayName` _asfirst_person_character) (`KismetSystemLibrary.IsValid` _asfirst_person_character))))
        (:`CastFailed`
          (`KismetSystemLibrary.PrintString` null "Invalid character data."))))
    (:`then_1`
      ;[1 1 1] Serialize movable static meshes, such as physics siimulations.
      (bind _outactors (`GameplayStatics.GetAllActorsOfClass` null "/Script/Engine.StaticMeshActor"))
      (for _array_element _outactors
        (if true
          (bind _returnvalue (`KismetSystemLibrary.GetObjectName` _array_element))
          (bind _returnvalue_2 (`KismetSystemLibrary.IsValid` _array_element))
          (`KismetArrayLibrary.Array_Add` (`local.MovableMeshes`) (make `/Game/Checkpoints/EmbeddedData/S_PhysicsMesh_Data` _returnvalue (`Actor.GetTransform` _array_element) (`SceneComponent.IsAnySimulatingPhysics` (`StaticMeshActor.StaticMeshComponent` _array_element)) (`Actor.GetVelocity` _array_element) _returnvalue_2))
          (`KismetSystemLibrary.PrintString` null (`KismetStringLibrary.BuildString_Bool` _returnvalue ", Valid = " _returnvalue_2 ".") false))))
    (:`then_2`
      ;[1 1 1] Serialize interactables.
      (bind _outactors_2 (`GameplayStatics.GetAllActorsOfClass` null "/Game/PlayerInteractables/BP_BasePlayerInteractable.BP_BasePlayerInteractable_C"))
      (for _array_element_2 _outactors_2
        (bind _returnvalue_3 (`KismetSystemLibrary.GetObjectName` _array_element_2))
        (bind _isactivated (`/Game/PlayerInteractables/BP_BasePlayerInteractable.isActivated` _array_element_2))
        (`KismetArrayLibrary.Array_Add` (`local.Interactables`) (make `/Game/Checkpoints/EmbeddedData/S_Interactable_Data` _returnvalue_3 _isactivated (`KismetSystemLibrary.IsValid` _array_element_2)))
        (`KismetSystemLibrary.PrintString` null (`KismetStringLibrary.BuildString_Bool` _returnvalue_3 ", State = " _isactivated ".") false)))
    (:`then_3`
      ;[1 1 1] Placeholder if anything else needs saving.
      (bind _asbp_my_game_mode (cast `/Game/UI/BP_MyGameMode` (`GameplayStatics.GetGameMode` null))
        (:`then`
          (set `local.timeSave` (make `/Game/Checkpoints/EmbeddedData/S_TimerSaveData` (`/Game/UI/BP_MyGameMode.Minutes` _asbp_my_game_mode) (`/Game/UI/BP_MyGameMode.Seconds` _asbp_my_game_mode) 0.0 true)))
        (:`CastFailed`
          (set `local.timeSave` (make `/Game/Checkpoints/EmbeddedData/S_TimerSaveData` 0)))))
    (:`then_4`
      (bind _outactors_3 (`GameplayStatics.GetAllActorsOfClass` null "/Game/Traps/ArrowTrap/BP_ArrowTrap.BP_ArrowTrap_C"))
      (for _array_element_3 _outactors_3
        (`KismetArrayLibrary.Array_Add` (`local.ArrowTrapSaves`) (make `/Game/Checkpoints/EmbeddedData/S_ArrowTrapData` false (`/Game/Traps/ArrowTrap/BP_ArrowTrap.TriggerInteractable` _array_element_3) (`KismetSystemLibrary.GetObjectName` _array_element_3)))))
    (:`then_5`
      ;[1 1 1] Put serialized data into save file and put it onto disk.
      (bind _returnvalue_4 (`GameplayStatics.CreateSaveGameObject` "/Game/Checkpoints/BP_TGS_Checkpoint_SaveGame.BP_TGS_Checkpoint_SaveGame_C"))
      (set `/Game/Checkpoints/BP_TGS_Checkpoint_SaveGame.Player Data` (`local.Player Data`) _returnvalue_4)
      (set `/Game/Checkpoints/BP_TGS_Checkpoint_SaveGame.Interactables` (`local.Interactables`) _returnvalue_4)
      (set `/Game/Checkpoints/BP_TGS_Checkpoint_SaveGame.NonStatic Meshes` (`local.MovableMeshes`) _returnvalue_4)
      (bind _returnvalue_5 (`GameplayStatics.SaveGameToSlot` _returnvalue_4 (`/Game/Checkpoints/BP_TGS_Checkpoint_SaveGame.Slot Name` _returnvalue_4) (`/Game/Checkpoints/BP_TGS_Checkpoint_SaveGame.Slot Number` _returnvalue_4)))
      (if _returnvalue_5
        (`KismetSystemLibrary.PrintString` null "Done!")
        (else
          (`KismetSystemLibrary.PrintString` null "Error Saving." true true (struct :`R` 1.0 :`B` 0.113637 :`A` 1.0)))))))