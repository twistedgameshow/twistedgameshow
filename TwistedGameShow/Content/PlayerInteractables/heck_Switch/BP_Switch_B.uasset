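; BP_Switch_B is a puzzle switch whose handle rotation and material reflect its IsActivated state.
; Updating eases the handle between upright and 90-degree pitch along the shortest path and swaps the mesh's activated or deactivated material.
; DeactivateSwitch clears the state and runs that same visual update.
; UpdateAfterChange refreshes the visuals, then has the PuzzleController check switch states.
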(event `Deactivate Switch`
  (bind _handle (`self.Handle`))
  (set `self.isActivated` false)
  (`KismetSystemLibrary.MoveComponentTo` _handle (`SceneComponent.RelativeLocation` _handle) (select `bool` (`self.isActivated`) :`true` (struct :`Roll` 90.0) :!type "Rotator Structure") true true 0.2 true :!label _label)
  (`PrimitiveComponent.SetMaterial` (`self.StaticMesh`) (`self.MaterialIndexToChange`) (select `bool` (`self.isActivated`) :`false` (`self.DeactivatedMaterial`) :`true` (`self.ActivatedMaterial`) :!type "MaterialInterface Object Reference")))

(event `self.UpdateAfterChange`
  (`self.Update Switch`)
  (`/Game/_MyContent/Dan/BP_SwitchPuzzleController.CheckSwitchStates` (`self.PuzzleController`)))

(event `Update Switch`
  (goto _label))

(fn `UserConstructionScript`
  (`parent.UserConstructionScript`))