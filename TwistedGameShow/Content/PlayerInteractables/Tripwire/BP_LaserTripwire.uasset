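; BP_LaserTripwire is a laser tripwire interactable that switches on while something overlaps it.
; Overlap begin calls Activate and overlap end calls Deactivate, for the first-person character or for any actor when CanBePressedByObjectsAsWell is set.
; Each end overlap deactivates it directly, with no count of remaining overlapping actors.
; The construction script only runs the parent's version.
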(event `self.ReceiveActorBeginOverlap`
  (params (OtherActor :type "Actor Object Reference"))
  (if (or (`.bSuccess` (cast `/Game/FirstPersonBP/Blueprints/FirstPersonCharacter` OtherActor :!pure true)) (`self.CanBePressedByObjectsAsWell`))
    (`self.Activate`)))

(event `self.ReceiveActorEndOverlap`
  (params (OtherActor :type "Actor Object Reference"))
  (if (or (`.bSuccess` (cast `/Game/FirstPersonBP/Blueprints/FirstPersonCharacter` OtherActor :!pure true)) (`self.CanBePressedByObjectsAsWell`))
    (`self.Deactivate`)))

(fn `UserConstructionScript`
  (`parent.UserConstructionScript`))